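; Artefact actor that continuously spins its ApoSMCroix component on roll, pitch and yaw together.
; Tick accumulates elapsed time and sets the relative rotation from it, with speed blended between slow and fast by the Active value.
; BeginPlay and actor overlap both set Active to full, and nothing connected lowers it, so it always spins at the fast rate.
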(event `self.ReceiveBeginPlay`
  (set `self.Active` 1.0))

(event `self.ReceiveActorBeginOverlap`
  (params (OtherActor :type "Actor Object Reference"))
  (set `self.Active` 1.0))

(event `self.ReceiveTick`
  (params (DeltaSeconds :type "Float (single-precision)"))
  (bind _returnvalue (* (* (`self.Time`) 360.0) (`KismetMathLibrary.Lerp` 1.0 10.0 (`self.Active`))))
  (set `self.Time` (+ DeltaSeconds (`self.Time`)))
  (`SceneComponent.K2_SetRelativeRotation` (`self.apo_SM_Croix`) (`KismetMathLibrary.MakeRotator` _returnvalue _returnvalue _returnvalue) false false))

(fn `UserConstructionScript`)