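; Artifact actor Blueprint whose core mesh, EMDSMCore, spins continuously on all three axes.
; Each tick accumulates time and sets the mesh's relative roll, pitch and yaw from it.
; Begin and end overlap toggle an Active value that doubles the multiplier while set.
; The multiplier scales total elapsed time, so orientation jumps on each toggle instead of only changing speed.
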(event `self.ReceiveActorEndOverlap`
  (params (OtherActor :type "Actor Object Reference"))
  (set `self.Active` 0.0))

(event `self.ReceiveActorBeginOverlap`
  (params (OtherActor :type "Actor Object Reference"))
  (set `self.Active` 1.0))

(event `self.ReceiveTick`
  (params (DeltaSeconds :type "Float (single-precision)"))
  (bind _returnvalue (* (* (`self.Time`) 150.0) (`KismetMathLibrary.Lerp` 1.0 2.0 (`self.Active`))))
  (set `self.Time` (+ DeltaSeconds (`self.Time`)))
  (`SceneComponent.K2_SetRelativeRotation` (`self.EMD_SM_Core`) (`KismetMathLibrary.MakeRotator` _returnvalue _returnvalue _returnvalue) false false))

(fn `UserConstructionScript`)