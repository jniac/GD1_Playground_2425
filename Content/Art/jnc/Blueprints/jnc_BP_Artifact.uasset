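; Artifact actor with a Core component that spins continuously and becomes faster and larger when activated.
; Beginning an overlap or pressing X plays a timeline that drives an Active value, and ending the overlap reverses it.
; Tick accumulates a custom time at a rate blended by Active, using it for three-axis rotation while Active also blends the Core's scale.
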(event `self.ReceiveBeginPlay`
  (`self.EnableInput` (`GameplayStatics.GetPlayerController` 0)))

(event `Key|X`
  (params (Key :type "Key Structure"))
  (:`Pressed`
    (bind (_direction _fifou) (`Timeline|Timeline` :!label _label)
      (:`Update`
        (set `self.active` _fifou)))))

(event `self.ReceiveActorBeginOverlap`
  (params (OtherActor :type "Actor Object Reference"))
  (goto _label))

(event `self.ReceiveActorEndOverlap`
  (params (OtherActor :type "Actor Object Reference"))
  (goto _label :!via `Reverse`))

(event `self.ReceiveTick`
  (params (DeltaSeconds :type "Float (single-precision)"))
  (bind _returnvalue (* (`self.time`) 30.0))
  (set `self.time` (+ (* DeltaSeconds (`KismetMathLibrary.Lerp` 1.0 10.0 (`self.active`))) (`self.time`)))
  ; Rotation
  (`SceneComponent.K2_SetRelativeRotation` (`self.core`) (`KismetMathLibrary.MakeRotator` _returnvalue _returnvalue _returnvalue) false false)
  ; Échelle
  (`SceneComponent.SetRelativeScale3D` (`self.core`) (`KismetMathLibrary.Conv_DoubleToVector` (`KismetMathLibrary.Lerp` 0.2 0.3 (`self.active`)))))

(fn `UserConstructionScript`)