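; Animated checkpoint actor that registers itself with the platformer game mode on overlap and exposes an arrow transform as its checkpoint info.
; Game mode checkpoint changes play its level sequence forward when it becomes current, or in reverse when replaced.
; A runtime-created sequence player binds to the actor and can drive the Opening and LateralActivation values.
; Tick and construction apply these to meshes, lights, materials and Niagara, alongside constantly spinning beams.
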(event `self.ReceiveBeginPlay`
  (set `self.opening` 0.0)
  (set `self.lateralActivation` 0.0)
  (`self.Update` 0.0)
  (`self.CreateSequencePlayer`)
  (add `/Game/Art/sdc/sdc_BP_PlatformerGameMode.CheckpointHasChanged` (`self.PlatformerGameMode`) (delegate `CheckpointHasChanged_Event`)))

(event `CheckpointHasChanged_Event`
  (params (newCheckpoint :type "/Game/Art/sdc/sdc_BPI_CheckpointActor Interface") (previousCheckpoint :type "/Game/Art/sdc/sdc_BPI_CheckpointActor Interface"))
  (if (`self.ShouldActivate` newCheckpoint previousCheckpoint)
    (`MovieSceneSequencePlayer.Play` (`self.levelSequence`))
    (elif (`self.ShouldDeactivate` newCheckpoint previousCheckpoint)
      (`MovieSceneSequencePlayer.PlayReverse` (`self.levelSequence`)))))

(event `self.ReceiveActorBeginOverlap`
  (params (OtherActor :type "Actor Object Reference"))
  (`/Game/Art/sdc/sdc_BP_PlatformerGameMode.SetCheckpoint` (`self.PlatformerGameMode`) self))

(event `self.ReceiveTick`
  (params (DeltaSeconds :type "Float (single-precision)"))
  (`self.Update` DeltaSeconds))

(fn `CheckpointInfo`
  (returns (transform :type "Transform Structure") (actor :type "Actor Object Reference"))
  (return (`SceneComponent.K2_GetComponentToWorld` (`self.Arrow`)) self))

(fn `CreateSequencePlayer`
  (bind (_outactor _returnvalue) (`LevelSequencePlayer.CreateLevelSequencePlayer` "/Game/Art/jnc/Misc/jnc_LS_Checkpoint.jnc_LS_Checkpoint" (make `MovieSceneSequencePlaybackSettings` false (struct) (struct :`bAllowRounding` true) 1.0 0.0 false false false false false false "ForceKeepState" true)))
  (`LevelSequenceActor.AddBinding` _outactor (`|GetSequenceBinding` null) self false)
  (set `self.levelSequence` _returnvalue))

(fn `PlatformerGameMode`
  (returns (platformerGameMode :type "/Game/Art/sdc/sdc_BP_PlatformerGameMode Object Reference"))
  (bind _assdc_bp_platformer_game_mode (cast `/Game/Art/sdc/sdc_BP_PlatformerGameMode` (`GameplayStatics.GetGameMode`))
    (:`then`
      _)
    (:`CastFailed`
      _))
  (return _assdc_bp_platformer_game_mode))

(fn `ShouldActivate`
  (params (newCheckpoint :type "/Game/Art/sdc/sdc_BPI_CheckpointActor Interface") (previousCheckpoint :type "/Game/Art/sdc/sdc_BPI_CheckpointActor Interface"))
  (returns (shouldActivate :type Boolean))
  (if true
    (bind (_transform _actor) (`/Game/Art/sdc/sdc_BPI_CheckpointActor.CheckpointInfo` (`local.newCheckpoint`)))
    (return (== _actor self))
    (else
      (return false))))

(fn `ShouldDeactivate`
  (params (newCheckpoint :type "/Game/Art/sdc/sdc_BPI_CheckpointActor Interface") (previousCheckpoint :type "/Game/Art/sdc/sdc_BPI_CheckpointActor Interface"))
  (returns (ShouldDeactivate :type Boolean))
  (if (`KismetSystemLibrary.IsValidInterface` (`local.previousCheckpoint`))
    (bind (_transform _actor) (`/Game/Art/sdc/sdc_BPI_CheckpointActor.CheckpointInfo` (`local.previousCheckpoint`)))
    (return (== _actor self))
    (else
      (return false))))

(fn `Update`
  (params (deltaTime :type "Float (double-precision)"))
  ; Permanent Animation
  (`self.UpdateBeams` deltaTime)
  ; Can be controlled by Level Sequence Player
  (`self.UpdateOpening`)
  (`self.UpdateLateralActivation`))

(fn `UpdateBeams`
  (params (deltaTime :type "Float (double-precision)"))
  (bind _array (`|MakeArray` (`self.RadialBeam`) (`self.RadialBeam1`) (`self.RadialBeam2`)))
  (set `self.beamTime` (+ (* deltaTime (`self.beamTimeScale`)) (`self.beamTime`)))
  (for (_array_element _array_index) _array
    (`SceneComponent.K2_SetRelativeRotation` _array_element (`KismetMathLibrary.MakeRotator` 0.0 0.0 (+ (* (`self.beamTime`) (`self.beamAngleVelocity`) -1.0) (* (- (`KismetArrayLibrary.Array_Length` _array) _array_index 1) (`self.beamAngleOffset`)))) false false)))

(fn `UpdateLateralActivation`
  (`SceneComponent.SetVisibility` (`self.LateralPanel`) (> (`self.lateralActivation`) 0.0) false)
  (`SceneComponent.SetVisibility` (`self.LateralPanel1`) (> (`self.lateralActivation`) 0.0) false)
  (`MeshComponent.SetScalarParameterValueOnMaterials` (`self.LateralPanel`) "Opacity" (`self.lateralActivation`))
  (`MeshComponent.SetScalarParameterValueOnMaterials` (`self.LateralPanel1`) "Opacity" (`self.lateralActivation`))
  (`LightComponent.SetIntensity` (`self.LateralLight`) (`KismetMathLibrary.Lerp` 0.0 2500.0 (`self.lateralActivation`))))

(fn `UpdateOpening`
  (`SceneComponent.K2_SetRelativeLocation` (`self.TopScene`) (`KismetMathLibrary.MakeVector` 0.0 0.0 (`KismetMathLibrary.Lerp` 100.0 300.0 (`self.opening`))) false false)
  (`SceneComponent.SetRelativeScale3D` (`self.NeonTube`) (`KismetMathLibrary.MakeVector` 0.75 0.75 (`KismetMathLibrary.Lerp` 0.0 2.0 (`self.opening`))))
  (`SceneComponent.SetRelativeScale3D` (`self.NeonTube1`) (`KismetMathLibrary.MakeVector` 0.75 0.75 (`KismetMathLibrary.Lerp` 0.0 2.0 (`self.opening`))))
  (`SceneComponent.SetRelativeScale3D` (`self.NeonTube2`) (`KismetMathLibrary.MakeVector` 0.75 0.75 (`KismetMathLibrary.Lerp` 0.0 2.0 (`self.opening`))))
  (`SceneComponent.SetRelativeScale3D` (`self.NeonTube3`) (`KismetMathLibrary.MakeVector` 0.75 0.75 (`KismetMathLibrary.Lerp` 0.0 2.0 (`self.opening`))))
  (`LightComponent.SetIntensity` (`self.PointLight`) (`KismetMathLibrary.Lerp` 500.0 5000.0 (`self.opening`)))
  (`SceneComponent.K2_SetRelativeLocation` (`self.PointLight`) (`KismetMathLibrary.MakeVector` 0.0 0.0 (`KismetMathLibrary.Lerp` 12.0 249.0 (`self.opening`))) false false)
  (set `self.beamTimeScale` (`KismetMathLibrary.Lerp` 1.0 3.0 (`self.opening`)))
  (set `self.beamAngleOffset` (`KismetMathLibrary.Lerp` 5.0 20.0 (`self.opening`)))
  (`ActorComponent.SetActive` (`self.jnc_NS_CheckpointOpen`) (> (`self.opening`) 0.2) false)
  (`SceneComponent.SetRelativeScale3D` (`self.jnc_NS_CheckpointOpen`) (`KismetMathLibrary.MakeVector` 1.0 1.0 (`KismetMathLibrary.Lerp` 0.0 1.0 (`self.opening`))))
  (`MeshComponent.SetScalarParameterValueOnMaterials` (`self.RadialBeam`) "Intensity" (`KismetMathLibrary.Lerp` 0.0 1.0 (`self.opening`)))
  (`MeshComponent.SetScalarParameterValueOnMaterials` (`self.RadialBeam1`) "Intensity" (`KismetMathLibrary.Lerp` 0.0 1.0 (`self.opening`)))
  (`MeshComponent.SetScalarParameterValueOnMaterials` (`self.RadialBeam2`) "Intensity" (`KismetMathLibrary.Lerp` 0.0 1.0 (`self.opening`))))

(fn `UserConstructionScript`
  (`self.Update` 0.0))