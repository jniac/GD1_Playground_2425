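; Jump pad actor that launches any overlapping Character upward to reach a configurable JumpHeight.
; On overlap it derives the Z launch velocity from the character's gravity scale, a fixed gravity constant and JumpHeight plus a small margin, overriding current vertical velocity.
; The construction script writes JumpHeight onto a text component so the value shows on the placed actor.
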(event `self.ReceiveBeginPlay`)

(event `self.ReceiveActorBeginOverlap`
  (params (OtherActor :type "Actor Object Reference"))
  (bind _ascharacter (cast `Character` OtherActor))
  (`Character.LaunchCharacter` _ascharacter (`KismetMathLibrary.MakeVector` 0.0 0.0 (`KismetMathLibrary.Sqrt` (* (* (`CharacterMovementComponent.GravityScale` (`Character.CharacterMovement` _ascharacter)) 980.0) (+ (`self.jumpHeight`) 50.0) 2.0))) false true))

(fn `UserConstructionScript`
  (`TextRenderComponent.K2_SetText` (`self.Text`) (`KismetTextLibrary.Conv_DoubleToText` (`self.jumpHeight`) "HalfToEven")))