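; Trigger actor that runs a mouse demo when something overlaps it, without filtering the overlapping actor.
; After a brief delay it shows the cursor, swaps input from the player to itself and displays the Jnc_W_MouseDemo widget.
; A timeline simultaneously glides the player character to the Arrow component's location.
; The widget's Done event or Space bar hides the cursor, restores player input and removes the widget.
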(event `self.ReceiveActorBeginOverlap`
  (params (OtherActor :type "Actor Object Reference"))
  (bind _returnvalue (`GameplayStatics.GetPlayerCharacter` 0))
  (`KismetSystemLibrary.Delay` 0.075)
  (set `PlayerController.bShowMouseCursor` true (`GameplayStatics.GetPlayerController` 0))
  (`self.DisableInput` (`GameplayStatics.GetPlayerCharacter` 0) null)
  (`self.DisableInput` (`GameplayStatics.GetPlayerController` 0) null)
  (`self.EnableInput` (`GameplayStatics.GetPlayerController` 0))
  (bind _returnvalue_2 (`|CreateWidget` "/Game/Art/jnc/Blueprints/jnc_W_MouseDemo.jnc_W_MouseDemo_C"))
  (add `/Game/Art/jnc/Blueprints/jnc_W_MouseDemo.Done` _returnvalue_2 (delegate `Done_Event`))
  (bind _output_get (set `self.widget` _returnvalue_2))
  (`UserWidget.AddToViewport` _output_get 0)
  (set `self.startLocation` (`self.K2_GetActorLocation` _returnvalue))
  (bind (_direction _alpha) (`Timeline|Timeline` :!via `PlayFromStart`)
    (:`Update`
      (`self.K2_SetActorLocation` _returnvalue (`KismetMathLibrary.VLerp` (`self.startLocation`) (`SceneComponent.K2_GetComponentLocation` (`self.Arrow`)) _alpha) false false))))

(event `Done_Event`
  (set `PlayerController.bShowMouseCursor` false (`GameplayStatics.GetPlayerController` 0) :!label _label)
  (`self.DisableInput` (`GameplayStatics.GetPlayerController` 0))
  (`self.EnableInput` (`GameplayStatics.GetPlayerController` 0) null)
  (`self.EnableInput` (`GameplayStatics.GetPlayerCharacter` 0) null)
  (`Widget.RemoveFromParent` (`self.widget`)))

(event `Key|SpaceBar`
  (params (Key :type "Key Structure"))
  (:`Pressed`
    (goto _label)))

(event `self.ReceiveActorEndOverlap`
  (params (OtherActor :type "Actor Object Reference")))

(fn `UserConstructionScript`)