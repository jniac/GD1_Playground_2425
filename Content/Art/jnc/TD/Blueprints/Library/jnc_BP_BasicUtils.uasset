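; Blueprint function library of basic math and hierarchy utilities.
; RoundBy and FloorBy snap each axis of a vector to multiples of a step.
; OnCircle converts an angle in degrees and a radius into a point on an origin-centered circle in the XY, YZ or XZ plane.
; IsChildOf walks up the attach-parent chain to test whether one component descends from another, optionally counting itself.
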(fn `FloorBy`
  (params (value :type "Vector Structure") (step :type "Float (double-precision)" :default 1.0))
  (returns (result :type "Vector Structure"))
  (return (* (`KismetMathLibrary.MakeVector` (`KismetMathLibrary.Conv_IntToDouble` (`KismetMathLibrary.FFloor` (.x (/ value step)))) (`KismetMathLibrary.Conv_IntToDouble` (`KismetMathLibrary.FFloor` (.y (/ value step)))) (`KismetMathLibrary.Conv_IntToDouble` (`KismetMathLibrary.FFloor` (.z (/ value step))))) (`local.step`))))

(fn `IsChildOf`
  (params (child :type "SceneComponent Object Reference") (parent :type "SceneComponent Object Reference") (includeSelf :type Boolean :default true))
  (returns (result :type Boolean))
  (locals (scope :type "SceneComponent Object Reference"))
  (if (and (== child parent) includeSelf)
    (return true)
    (else
      (set `local.scope` (`SceneComponent.GetAttachParent` (`local.child`)))
      (while (`KismetSystemLibrary.IsValid` (`local.scope`))
        (if (== (`local.scope`) (`local.parent`))
          (return true)
          (else
            (set `local.scope` (`SceneComponent.GetAttachParent` (`local.scope`))))))
      (return false))))

(fn `OnCircle`
  (params (angle :type "Float (double-precision)") (radius :type "Float (double-precision)" :default 100.0) (plane :type "/Game/Art/jnc/TD/Blueprints/jnc_E_Plane Enum" :default "NewEnumerator0"))
  (returns (point :type "Vector Structure"))
  (bind _returnvalue (`KismetMathLibrary.DegreesToRadians` angle))
  (bind _returnvalue_2 (* (`KismetMathLibrary.Sin` _returnvalue) (`local.radius`)))
  (bind _returnvalue_3 (* (`KismetMathLibrary.Cos` _returnvalue) (`local.radius`)))
  (switch `/Game/Art/jnc/TD/Blueprints/jnc_E_Plane` plane
    (:`NewEnumerator0`
      (return (`KismetMathLibrary.MakeVector` _returnvalue_3 _returnvalue_2)))
    (:`NewEnumerator1`
      (return (`KismetMathLibrary.MakeVector` 0.0 _returnvalue_3 _returnvalue_2)))
    (:`NewEnumerator2`
      (return (`KismetMathLibrary.MakeVector` _returnvalue_3 0.0 _returnvalue_2)))))

(fn `RoundBy`
  (params (value :type "Vector Structure") (step :type "Float (double-precision)" :default 1.0))
  (returns (result :type "Vector Structure"))
  (return (* (`KismetMathLibrary.MakeVector` (`KismetMathLibrary.Conv_IntToDouble` (`KismetMathLibrary.Round` (.x (/ value step)))) (`KismetMathLibrary.Conv_IntToDouble` (`KismetMathLibrary.Round` (.y (/ value step)))) (`KismetMathLibrary.Conv_IntToDouble` (`KismetMathLibrary.Round` (.z (/ value step))))) (`local.step`))))