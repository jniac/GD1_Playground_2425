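; Blueprint function library of easing and remapping math helpers.
; InverseLerp normalizes a value within a range and clamps it, building on an unclamped variant.
; InOut is a power-based ease-in/ease-out curve with an adjustable inflection point, ported from the linked some-utils-ts transition code.
; RemapInOut chains both to map an input range onto an output range with that easing.
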(fn `InOut`
  (params (x :type "Float (double-precision)") (power :type "Float (double-precision)" :default 3.0) (inflection :type "Float (double-precision)" :default 0.333333))
  (returns (value :type "Float (double-precision)"))
  ; https://github.com/jniac/some-utils-ts/blob/main/src/math/easing/transition.ts#L19-L33
  (if (<= (`local.x`) 0.0)
    (return 0.0)
    (elif (>= (`local.x`) 1.0)
      (return 1.0)
      (elif (<= (`local.x`) (`local.inflection`))
        (return (* (/ 1.0 (`KismetMathLibrary.MultiplyMultiply_FloatFloat` (`local.inflection`) (- (`local.power`) 1.0))) (`KismetMathLibrary.MultiplyMultiply_FloatFloat` (`local.x`) (`local.power`))))
        (else
          (return (- 1.0 (* (/ 1.0 (`KismetMathLibrary.MultiplyMultiply_FloatFloat` (- 1.0 (`local.inflection`)) (- (`local.power`) 1.0))) (`KismetMathLibrary.MultiplyMultiply_FloatFloat` (- 1.0 (`local.x`)) (`local.power`))))))))))

(fn `InverseLerp`
  (params (a :type "Float (double-precision)") (b :type "Float (double-precision)") (alpha :type "Float (double-precision)"))
  (returns (value :type "Float (double-precision)"))
  (return (`KismetMathLibrary.FClamp` (`self.InverseLerpUnclamped` a b alpha))))

(fn `InverseLerpUnclamped`
  (params (a :type "Float (double-precision)") (b :type "Float (double-precision)") (alpha :type "Float (double-precision)"))
  (returns (value :type "Float (double-precision)"))
  (return (/ (- alpha a) (- b a))))

(fn `RemapInOut`
  (params (alpha :type "Float (double-precision)") (inA :type "Float (double-precision)") (inB :type "Float (double-precision)" :default 1.0) (outA :type "Float (double-precision)") (outB :type "Float (double-precision)" :default 1.0) (power :type "Float (double-precision)" :default 3.0) (inflection :type "Float (double-precision)" :default 0.333333))
  (returns (value :type "Float (double-precision)"))
  (return (`KismetMathLibrary.Lerp` outA outB (`self.InOut` (`self.InverseLerp` inA inB alpha) power inflection))))