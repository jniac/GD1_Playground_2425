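; Actor component that exposes an observable boolean value to its owning actor.
; On BeginPlay it constructs a Jnc_ObservableBool object and forwards Get and Set to it, returning current and previous values plus whether a change occurred.
; Tick accumulates a local clock that is passed to Set as the timestamp, letting ElapsedTime report the seconds since the recorded change.
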(event `self.ReceiveBeginPlay`
  (bind _returnvalue (`|GenericCreateObject` "/Game/Art/jnc/TD/Blueprints/Observables/jnc_ObservableBool.jnc_ObservableBool_C"))
  (set `self.obs` _returnvalue))

(event `self.ReceiveTick`
  (params (DeltaSeconds :type "Float (single-precision)"))
  (set `self.time` (+ (`self.time`) DeltaSeconds)))

(fn `ElapsedTime`
  (returns (elapsed :type "Float (double-precision)"))
  (return (- (`self.time`) (`/Game/Art/jnc/TD/Blueprints/Observables/jnc_ObservableBool._changeTime` (`self.obs`)))))

(fn `Get`
  (returns (value :type Boolean) (valueOld :type Boolean))
  (bind (_value _valueold) (`/Game/Art/jnc/TD/Blueprints/Observables/jnc_ObservableBool.Get` (`self.obs`)))
  (return _value _valueold))

(fn `Set`
  (params (newValue :type Boolean))
  (returns (hasChanged :type Boolean) (value :type Boolean) (valueOld :type Boolean))
  (bind (_haschanged _value _valueold) (`/Game/Art/jnc/TD/Blueprints/Observables/jnc_ObservableBool.Set` (`self.obs`) newValue (`self.time`)))
  (return _haschanged _value _valueold))