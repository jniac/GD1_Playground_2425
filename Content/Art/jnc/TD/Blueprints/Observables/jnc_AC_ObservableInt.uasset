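; Actor component that holds an observable integer for its owning actor.
; On BeginPlay it constructs a Jnc_ObservableInt object and resets it to an initial value, then forwards Get and Set to it, returning current and previous values.
; Tick accumulates a local time, which Set passes to the object so ElapsedTime can report seconds since its recorded change time.
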(event `self.ReceiveBeginPlay`
  (bind _returnvalue (`|GenericCreateObject` "/Game/Art/jnc/TD/Blueprints/Observables/jnc_ObservableInt.jnc_ObservableInt_C"))
  (bind _output_get (set `self.obs` _returnvalue))
  (`/Game/Art/jnc/TD/Blueprints/Observables/jnc_ObservableInt.Reset` _output_get (`self.initialValue`)))

(event `self.ReceiveTick`
  (params (DeltaSeconds :type "Float (single-precision)"))
  (set `self.time` (+ (`self.time`) DeltaSeconds)))

(fn `ElapsedTime`
  (returns (elapsed :type "Float (double-precision)"))
  (return (- (`self.time`) (`/Game/Art/jnc/TD/Blueprints/Observables/jnc_ObservableInt._changeTime` (`self.obs`)))))

(fn `Get`
  (returns (value :type Integer) (_valueOld :type Integer))
  (bind (_value __valueold) (`/Game/Art/jnc/TD/Blueprints/Observables/jnc_ObservableInt.Get` (`self.obs`)))
  (return _value __valueold))

(fn `Set`
  (params (newValue :type Integer))
  (returns (value :type Integer) (valueOld :type Integer))
  (bind (_value _valueold) (`/Game/Art/jnc/TD/Blueprints/Observables/jnc_ObservableInt.Set` (`self.obs`) newValue (`self.time`)))
  (return _value _valueold))