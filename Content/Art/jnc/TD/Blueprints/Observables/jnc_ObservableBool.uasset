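; Observable boolean object that stores a current value, previous value and change time, and notifies listeners when the value flips.
; Set always shifts the current value into the old one, but stamps the time and calls OnChange only on a real change.
; Reset goes through Set with a time of -1, then makes both values equal.
; Get reports the old value as the inverse of the current one, ignoring the stored copy.
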(fn `Get`
  (returns (value :type Boolean) (valueOld :type Boolean))
  (return (`self._value`) (not (`self._value`))))

(fn `Reset`
  (params (resetValue :type Boolean))
  (bind (_haschanged _value) (`self.Set` resetValue))
  (set `self._valueOld` _value))

(fn `Set`
  (params (newValue :type Boolean) (time :type "Float (double-precision)" :default -1.0))
  (returns (hasChanged :type Boolean) (value :type Boolean) (valueOld :type Boolean))
  (locals (_hasChanged :type Boolean))
  (set `local._hasChanged` (!= newValue (`self._value`)))
  ; May look overkill to keep a reference to the "old" value of a bool, since it's always the inverse value of the current value, but in fact, at the initialiazation (reset) value & valueOld must have the same value.
  (set `self._valueOld` (`self._value`))
  (set `self._value` (`local.newValue`))
  (if (`local._hasChanged`)
    (set `self._changeTime` (`local.time`))
    (`self.OnChange` (`self._value`) (`self._valueOld`) (`self._changeTime`)))
  (return (`local._hasChanged`) (`self._value`) (`self._valueOld`)))