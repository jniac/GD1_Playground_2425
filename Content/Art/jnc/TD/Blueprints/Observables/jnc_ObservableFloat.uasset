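; A Blueprint observable float that wraps a value and notifies listeners when it changes.
; Set stores the previous and new values, and on an actual change records the supplied time and fires OnChange with value, old value and change time.
; Get returns current and previous values, while Reset sets a value at time zero, then aligns the old value to it.
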(fn `Get`
  (returns (value :type "Float (double-precision)") (_valueOld :type "Float (double-precision)"))
  (return (`self._value`) (`self._valueOld`)))

(fn `Reset`
  (params (resetValue :type "Float (double-precision)"))
  (bind _value (`self.Set` resetValue))
  (set `self._valueOld` _value))

(fn `Set`
  (params (newValue :type "Float (double-precision)") (time :type "Float (double-precision)"))
  (returns (value :type "Float (double-precision)") (valueOld :type "Float (double-precision)") (hasChanged :type Boolean))
  (locals (_hasChanged :type Boolean))
  (set `local._hasChanged` (!= newValue (`self._value`)))
  (set `self._valueOld` (`self._value`))
  (set `self._value` (`local.newValue`))
  (if (`local._hasChanged`)
    (set `self._changeTime` (`local.time`))
    (`self.OnChange` (`self._value`) (`self._valueOld`) (`self._changeTime`)))
  (return (`self._value`) (`self._valueOld`) (`local._hasChanged`)))