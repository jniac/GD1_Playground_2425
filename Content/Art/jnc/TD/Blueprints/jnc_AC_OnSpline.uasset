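; jnc_AC_OnSpline is a component that moves its owning actor along a given spline at a set velocity.
; SetSplineToFollow stores the spline, caches its length and converts InitialTime, as a fraction of that length, into a starting distance.
; Each tick advances that distance and applies the spline's local-space transform, without scale, directly to the actor as its transform.
; The distance is never wrapped or clamped.
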(event `self.ReceiveTick`
  (params (DeltaSeconds :type "Float (single-precision)"))
  (`self.UpdatePosition` DeltaSeconds))

(fn `SetSplineToFollow`
  (params (splineToFollow :type "SplineComponent Object Reference") (initialTime :type "Float (double-precision)"))
  (bind _output_get (set `self.splineToFollow` splineToFollow))
  (`/Engine/EditorBlueprintResources/StandardMacros.IsValid` _output_get
    (:`Is Valid`
      (bind _output_get_2 (set `self.splineLength` (`SplineComponent.GetSplineLength` (`self.splineToFollow`))))
      (set `self.position` (* _output_get_2 (`local.initialTime`))))))

(fn `UpdatePosition`
  (params (deltaTime :type "Float (double-precision)"))
  (`/Engine/EditorBlueprintResources/StandardMacros.IsValid` (`self.splineToFollow`)
    (:`Is Valid`
      ; Update "position"
      (set `self.position` (+ (`self.position`) (* (`local.deltaTime`) (`self.velocity`))))
      (`Actor.K2_SetActorTransform` (`self.GetOwner`) (`SplineComponent.GetTransformAtDistanceAlongSpline` (`self.splineToFollow`) (`self.position`) "Local" false) false false))))