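; Base card actor for a hand of cards, showing a widget sorted by card index and supporting dragging out of and back to its hand slot.
; An observable Dragged flag drives motion: while set, Tick places the card at hand position plus drag offset and eases its hand rotation to zero.
; On release, the Back timeline lerps the card from its current transform to the stored hand transform.
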(event `self.ReceiveBeginPlay`
  (add `/Game/Art/jnc/TD/Blueprints/Observables/jnc_ObservableBool.OnChange` (`/Game/Art/jnc/TD/Blueprints/Observables/AC/jnc_AC_ObservableBoolean.obs` (`self.dragged`)) (delegate `OnChange_Event`)))

(event `OnChange_Event`
  (params (value :type Boolean) (valueOld :type Boolean) (changeTime :type "Float (double-precision)"))
  (if (not value)
    (`self.BackToHand`)))

(event `BackToHand`
  (set `self.startTransform` (`SceneComponent.GetRelativeTransform` (`self.DefaultSceneRoot`)))
  (bind (_direction _alpha) (`Timeline|Back` :!via `PlayFromStart`)
    (:`Update`
      (`SceneComponent.K2_SetRelativeTransform` (`self.DefaultSceneRoot`) (`KismetMathLibrary.TLerp` (`self.startTransform`) (`self.handTransform`) _alpha) false false))))

(event `self.ReceiveTick`
  (params (DeltaSeconds :type "Float (single-precision)"))
  (bind (_handtransform_location _handtransform_rotation _handtransform_scale) (`KismetMathLibrary.BreakTransform` (`self.handTransform`)))
  (if (`/Game/Art/jnc/TD/Blueprints/Observables/AC/jnc_AC_ObservableBoolean.Get` (`self.dragged`))
    (`SceneComponent.K2_SetRelativeTransform` (`self.DefaultSceneRoot`) (`KismetMathLibrary.MakeTransform` (+ _handtransform_location (`self.Offset`)) (* _handtransform_rotation (`/Game/Art/jnc/TD/Blueprints/Library/jnc_BP_Easing.RemapInOut` (`/Game/Art/jnc/TD/Blueprints/Observables/AC/jnc_AC_ObservableBoolean.ElapsedTime` (`self.dragged`)) 0.0 0.3 1.0 0.0 5.0 0.2)) _handtransform_scale) false false)))

(fn `DragEnter`
  (`/Game/Art/jnc/TD/Blueprints/Observables/AC/jnc_AC_ObservableBoolean.Set` (`self.dragged`) true))

(fn `DragExit`
  (`/Game/Art/jnc/TD/Blueprints/Observables/AC/jnc_AC_ObservableBoolean.Set` (`self.dragged`) false))

(fn `InitializeCard`
  (params (handTransform :type "Transform Structure") (cardIndex :type Integer))
  (set `self.handTransform` handTransform)
  (bind _output_get (set `self.cardIndex` cardIndex))
  (`PrimitiveComponent.SetTranslucentSortPriority` (`self.Widget`) _output_get)
  (`SceneComponent.K2_SetRelativeTransform` (`self.DefaultSceneRoot`) handTransform false false))

(fn `SetDragOffset`
  (params (offset :type "Vector Structure"))
  (set `self.Offset` offset))

(fn `UserConstructionScript`)