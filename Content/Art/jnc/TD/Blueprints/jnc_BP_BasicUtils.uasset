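; jnc_BP_BasicUtils is a small utility Blueprint with two math helpers that snap vector values to multiples of a step.
; RoundBy snaps each of X, Y and Z to the nearest multiple, while FloorBy snaps each down to the multiple at or below it.
; Both divide by Step, convert each component to a whole number, rebuild the vector and multiply by Step again.
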(fn `FloorBy`
  (params (value :type "Vector Structure") (step :type "Float (double-precision)" :default 1.0))
  (returns (result :type "Vector Structure"))
  (return (* (`KismetMathLibrary.MakeVector` (`KismetMathLibrary.Conv_IntToDouble` (`KismetMathLibrary.FFloor` (.x (/ value step)))) (`KismetMathLibrary.Conv_IntToDouble` (`KismetMathLibrary.FFloor` (.y (/ value step)))) (`KismetMathLibrary.Conv_IntToDouble` (`KismetMathLibrary.FFloor` (.z (/ value step))))) (`local.step`))))

(fn `RoundBy`
  (params (value :type "Vector Structure") (step :type "Float (double-precision)" :default 1.0))
  (returns (result :type "Vector Structure"))
  (return (* (`KismetMathLibrary.MakeVector` (`KismetMathLibrary.Conv_IntToDouble` (`KismetMathLibrary.Round` (.x (/ value step)))) (`KismetMathLibrary.Conv_IntToDouble` (`KismetMathLibrary.Round` (.y (/ value step)))) (`KismetMathLibrary.Conv_IntToDouble` (`KismetMathLibrary.Round` (.z (/ value step))))) (`local.step`))))