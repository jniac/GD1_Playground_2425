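; Actor that displays a hand of up to ten cards fanned along an arc, enlarging the card under the player controller's hit component.
; CreateCards runs on construction and BeginPlay, rebuilding the hand as BasicCard child actors with stepped widget translucent sort priorities for layering.
; While a hit component is valid, Tick matches it to a card and eases every card's scale toward its highlighted or normal size.
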(event `self.ReceiveBeginPlay`
  (`self.CreateCards`))

(event `self.ReceiveTick`
  (params (DeltaSeconds :type "Float (single-precision)"))
  (bind _hitcomponent (`/Game/Art/jnc/TD/Blueprints/jnc_BP_TDPlayerController.hitComponent` (`/Game/Art/jnc/TD/Blueprints/Library/jnc_BP_TD_Utils.TD PlayerController`)))
  (`/Engine/EditorBlueprintResources/StandardMacros.IsValid` _hitcomponent
    (:`Is Valid`
      (set `self.cardIndex` (`self.GetHitCardIndex` _hitcomponent))
      (for (_array_element _array_index) (`self.cards`)
        (`SceneComponent.SetRelativeScale3D` _array_element (`KismetMathLibrary.VLerp` (`SceneComponent.RelativeScale3D` _array_element) (`KismetMathLibrary.Conv_DoubleToVector` (`KismetMathLibrary.SelectFloat` 1.1 1.0 (== _array_index (`self.cardIndex`)))) 0.2))))))

(fn `CreateCards`
  (bind _radius (`self.radius`))
  ; Safe check
  (set `self.cardCount` (`KismetMathLibrary.Clamp` (`self.cardCount`) 1 10))
  (`self.RemoveAllCards`)
  (for _index (range (`self.cardCount`))
    (bind _returnvalue (* (`self.angle`) (`KismetMathLibrary.Lerp` -1.0 1.0 (/ (`KismetMathLibrary.Conv_IntToDouble` _index) (- (`self.cardCount`) 1)))))
    (bind _returnvalue_2 (`AddComponent|NODE_AddChildActorComponent-0` :`RelativeTransform` (`KismetMathLibrary.MakeTransform` (+ (`/Game/Art/jnc/TD/Blueprints/Library/jnc_BP_BasicUtils.OnCircle` (+ _returnvalue 90.0) _radius "NewEnumerator1") (`KismetMathLibrary.MakeVector` 0.0 0.0 (* _radius -1.0))) (`KismetMathLibrary.MakeRotator` (+ (* _returnvalue -1.0) 3.0) 0.0 10.0))))
    (`|ExecutionSequence`
      (:`then_0`
        (`KismetArrayLibrary.Array_Add` (`self.cards`) _returnvalue_2))
      (:`then_1`
        (`ChildActorComponent.SetChildActorClass` _returnvalue_2 "/Game/Art/jnc/TD/Blueprints/jnc_BP_BasicCard.jnc_BP_BasicCard_C"))
      (:`then_2`
        (bind _asjnc_bp_basic_card (cast `/Game/Art/jnc/TD/Blueprints/jnc_BP_BasicCard` (`ChildActorComponent.ChildActor` _returnvalue_2)))
        (`PrimitiveComponent.SetTranslucentSortPriority` (`/Game/Art/jnc/TD/Blueprints/jnc_BP_BasicCard.Widget` _asjnc_bp_basic_card) (* _index 10))))))

(fn `GetHitCardIndex`
  (params (hitComponent :type "SceneComponent Object Reference"))
  (returns (index :type Integer))
  (for (_array_element _array_index) (`self.cards`)
    (if (`/Game/Art/jnc/TD/Blueprints/Library/jnc_BP_BasicUtils.IsChildOf` (`local.hitComponent`) _array_element)
      (return _array_index)))
  (return -1))

(fn `RemoveAllCards`
  (for _array_element (`self.cards`)
    (`ActorComponent.K2_DestroyComponent` _array_element))
  (`KismetArrayLibrary.Array_Clear` (`self.cards`)))

(fn `UserConstructionScript`
  (`self.CreateCards`))