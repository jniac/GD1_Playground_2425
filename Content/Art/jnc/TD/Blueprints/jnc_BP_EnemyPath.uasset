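; Enemy path actor that defines a route with a master spline and can draw it, along with a derived rounded version.
; The construction script optionally renders the master spline, then optionally creates a second spline component that RoundedSpline computes from the master.
; RenderSpline adds a cylinder spline mesh per segment, using straight-line tangents for linear or constant points and the points' own tangents for curves.
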(event `self.ReceiveBeginPlay`)

(fn `RenderSpline`
  (params (spline :type "SplineComponent Object Reference"))
  (locals (splineMesh :type "SplineMeshComponent Object Reference"))
  (bind _spline (`local.spline`))
  (bind _splinemesh (`local.splineMesh`))
  (bind _splinemesh_2 (`local.splineMesh`))
  (bind _splinemesh_3 (`local.splineMesh`))
  (for _index (range (`SplineComponent.GetNumberOfSplineSegments` spline))
    (bind _returnvalue (`AddComponent|NODE_AddSplineMeshComponent-0`))
    (set `local.splineMesh` _returnvalue)
    (`|ExecutionSequence`
      (:`then_0`
        (`StaticMeshComponent.SetStaticMesh` _splinemesh_3 "/Game/Art/jnc/TD/Meshes/jnc_SM_SplineCylinder.jnc_SM_SplineCylinder")
        (`SceneComponent.SetHiddenInGame` _splinemesh_3 false false))
      (:`then_1`
        (bind (_returnvalue_inputkey _returnvalue_position _returnvalue_arrivetangent _returnvalue_leavetangent _returnvalue_rotation _returnvalue_scale _returnvalue_type) (break `SplinePoint` (`SplineComponent.GetSplinePointAt` _spline _index "Local")))
        (`SplineMeshComponent.SetStartPosition` _splinemesh_2 _returnvalue_position false)
        (bind (_returnvalue_inputkey_2 _returnvalue_position_2 _returnvalue_arrivetangent_2 _returnvalue_leavetangent_2 _returnvalue_rotation_2 _returnvalue_scale_2 _returnvalue_type_2) (break `SplinePoint` (`SplineComponent.GetSplinePointAt` _spline (+ _index 1) "Local")))
        (bind _returnvalue_2 (- _returnvalue_position_2 _returnvalue_position))
        (`SplineMeshComponent.SetStartTangent` _splinemesh_2 (select `ESplinePointType` _returnvalue_type :`Linear` _returnvalue_2 :`Curve` _returnvalue_leavetangent :`Constant` _returnvalue_2 :`CurveClamped` _returnvalue_leavetangent :`CurveCustomTangent` _returnvalue_leavetangent) false))
      (:`then_2`
        (`SplineMeshComponent.SetEndPosition` _splinemesh _returnvalue_position_2 false)
        (`SplineMeshComponent.SetEndTangent` _splinemesh (select `ESplinePointType` _returnvalue_type_2 :`Linear` _returnvalue_2 :`Curve` _returnvalue_arrivetangent_2 :`Constant` _returnvalue_2 :`CurveClamped` _returnvalue_arrivetangent_2 :`CurveCustomTangent` _returnvalue_arrivetangent_2) true)))))

(fn `UserConstructionScript`
  (`|ExecutionSequence`
    (:`then_0`
      (`SceneComponent.SetHiddenInGame` (`self.Spline`) (not (`self.renderMasterSpline`)) false)
      (if (`self.renderMasterSpline`)
        (`self.RenderSpline` (`self.Spline`))))
    (:`then_1`
      (if (`self.renderDerivedSpline`)
        ;[0.005605 0.005605 0.005605] Create the "derived" spline component, and compute its points.
        (bind _returnvalue (`AddComponent|NODE_AddSplineComponent-1`))
        (set `self.DerivedSpline` _returnvalue)
        (`/Game/Art/jnc/TD/Blueprints/Library/jnc_BP_SplineUtils.RoundedSpline` 50.0 (`self.Spline`) (`self.DerivedSpline`))
        (`self.RenderSpline` (`self.DerivedSpline`))))))