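; Hand-of-cards actor that fans out card actors along an arc and handles cursor hover and dragging.
; Construction rebuilds a clamped number of jnc_BP_BasicCard child actors, each given a hand transform and index.
; Observable hover and down indices, fed by the TD player controller's hit component and cursor state, notify the affected cards.
; Tick eases the pressed card's scale up and offsets it by cursor trace movement in hand-local space.
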(event `self.ReceiveBeginPlay`
  (add `/jnc/Observables/jnc_ObservableBool.OnChange` (`/Game/Art/jnc/TD/Blueprints/jnc_BP_TDPlayerController.cursorIsDown` (`/Game/Art/jnc/TD/Blueprints/jnc_BP_TD_Utils.TD PlayerController`)) (delegate `OnChange_Event`))
  (add `/jnc/Observables/jnc_ObservableInt.OnChange` (`/jnc/Observables/AC/jnc_AC_ObservableInt.obs` (`self.hoverIndex`)) (delegate `Hover_OnChange_Event`)))

(event `OnChange_Event`
  (params (value :type Boolean) (valueOld :type Boolean) (changeTime :type "Float (double-precision)"))
  (`self.OnDownChange` value))

(event `Hover_OnChange_Event`
  (params (value :type Integer) (valueOld :type Integer) (changeTime :type "Float (double-precision)"))
  (`self.OnHoverIndexChange` value valueOld))

(event `self.ReceiveTick`
  (params (DeltaSeconds :type "Float (single-precision)"))
  (bind _returnvalue (`self.GetTransform`))
  (bind _value (`/jnc/Observables/AC/jnc_AC_ObservableInt.Get` (`self.downIndex`)))
  (`self.UpdateHoverIndex`)
  (`self.UpdateCardsScale`)
  (if (!= _value -1)
    (`/Game/Art/jnc/TD/Blueprints/jnc_BP_BasicCard.SetDragOffset` (`|GetArrayItem` (`self.cardActors`) _value) (/ (`KismetMathLibrary.InverseTransformDirection` _returnvalue (- (`self.GetDragPlaneImpactPoint`) (`self.impactOnDown`))) (.x (.scale _returnvalue))))))

(fn `CreateCards`
  (bind _radius (`self.radius`))
  ; Safe check
  (set `self.cardCount` (`KismetMathLibrary.Clamp` (`self.cardCount`) 1 10))
  (`self.RemoveAllCards`)
  (for _index (range (`self.cardCount`))
    (bind _returnvalue (`AddComponent|NODE_AddChildActorComponent-0`))
    (`KismetArrayLibrary.Array_Add` (`self.cards`) _returnvalue)
    (`ChildActorComponent.SetChildActorClass` _returnvalue "/Game/Art/jnc/TD/Blueprints/jnc_BP_BasicCard.jnc_BP_BasicCard_C")
    (bind _asjnc_bp_basic_card (cast `/Game/Art/jnc/TD/Blueprints/jnc_BP_BasicCard` (`ChildActorComponent.ChildActor` _returnvalue)))
    (bind _returnvalue_2 (* (`self.angle`) (`KismetMathLibrary.Lerp` -1.0 1.0 (/ (`KismetMathLibrary.Conv_IntToDouble` _index) (- (`self.cardCount`) 1)))))
    (`/Game/Art/jnc/TD/Blueprints/jnc_BP_BasicCard.InitializeCard` _asjnc_bp_basic_card (`KismetMathLibrary.MakeTransform` (+ (`/jnc/Library/jnc_BP_BasicUtils.OnCircle` (+ _returnvalue_2 90.0) _radius "NewEnumerator1") (`KismetMathLibrary.MakeVector` 0.0 0.0 (* _radius -1.0))) (`KismetMathLibrary.MakeRotator` (+ (* _returnvalue_2 -1.0) 3.0) 0.0 10.0)) _index)
    (`KismetArrayLibrary.Array_Add` (`self.cardActors`) _asjnc_bp_basic_card)))

(fn `CurrentDownCard`
  (returns (card :type "ChildActorComponent Object Reference") (cardActor :type "/Game/Art/jnc/TD/Blueprints/jnc_BP_BasicCard Object Reference"))
  (bind _value (`/jnc/Observables/AC/jnc_AC_ObservableInt.Get` (`self.downIndex`)))
  (if (!= _value -1)
    (return (`|GetArrayItem` (`self.cards`) _value) (`|GetArrayItem` (`self.cardActors`) _value))
    (else
      (return null null))))

(fn `CurrentDownCardOld`
  (returns (cardOld :type "ChildActorComponent Object Reference") (cardActorOld :type "/Game/Art/jnc/TD/Blueprints/jnc_BP_BasicCard Object Reference"))
  (bind (_value __valueold) (`/jnc/Observables/AC/jnc_AC_ObservableInt.Get` (`self.downIndex`)))
  (if (!= __valueold -1)
    (return (`|GetArrayItem` (`self.cards`) __valueold) (`|GetArrayItem` (`self.cardActors`) __valueold))
    (else
      (return null null))))

(fn `GetDragPlaneImpactPoint`
  (returns (ImpactPoint :type "Vector Structure") (hit :type Boolean))
  (bind (_hitresult _returnvalue) (`PlayerController.GetHitResultUnderCursorForObjects` (`/Game/Art/jnc/TD/Blueprints/jnc_BP_TD_Utils.TD PlayerController`) (`|MakeArray` "ObjectTypeQuery9" :!type "EObjectTypeQuery Enum") true))
  (return (`.ImpactPoint` (`GameplayStatics.BreakHitResult` _hitresult)) _returnvalue))

(fn `GetHitCardIndex`
  (params (hitComponent :type "SceneComponent Object Reference"))
  (returns (index :type Integer))
  (for (_array_element _array_index) (`self.cards`)
    (if (`/jnc/Library/jnc_BP_BasicUtils.IsChildOf` (`local.hitComponent`) _array_element)
      (return _array_index)))
  (return -1))

(fn `OnDownChange`
  (params (cursorDown :type Boolean))
  (bind (_card _cardactor) (`self.CurrentDownCard`))
  (bind (_cardold _cardactorold) (`self.CurrentDownCardOld`))
  (`/jnc/Observables/AC/jnc_AC_ObservableInt.Set` (`self.downIndex`) (`KismetMathLibrary.SelectInt` (`/jnc/Observables/AC/jnc_AC_ObservableInt.Get` (`self.hoverIndex`)) -1 cursorDown))
  (`/Engine/EditorBlueprintResources/StandardMacros.IsValid` _cardactorold
    (:`Is Valid`
      (`/Game/Art/jnc/TD/Blueprints/jnc_BP_BasicCard.DragExit` _cardactorold))
    (:`Is Not Valid`
      _))
  (`/Engine/EditorBlueprintResources/StandardMacros.IsValid` _cardactor
    (:`Is Valid`
      (`/Game/Art/jnc/TD/Blueprints/jnc_BP_BasicCard.DragEnter` _cardactor))
    (:`Is Not Valid`
      _))
  (if (`local.cursorDown`)
    (set `self.impactOnDown` (`self.GetDragPlaneImpactPoint`))))

(fn `OnHoverIndexChange`
  (params (index :type Integer) (indexOld :type Integer))
  (bind _output (`|GetArrayItem` (`self.cardActors`) index))
  (bind _output_2 (`|GetArrayItem` (`self.cardActors`) (`local.indexOld`)))
  (`/Engine/EditorBlueprintResources/StandardMacros.IsValid` _output
    (:`Is Valid`
      (`/jnc/Observables/AC/jnc_AC_ObservableBoolean.Set` (`/Game/Art/jnc/TD/Blueprints/jnc_BP_BasicCard.hovered` _output) true))
    (:`Is Not Valid`
      _))
  (`/Engine/EditorBlueprintResources/StandardMacros.IsValid` _output_2
    (:`Is Valid`
      (`/jnc/Observables/AC/jnc_AC_ObservableBoolean.Set` (`/Game/Art/jnc/TD/Blueprints/jnc_BP_BasicCard.hovered` _output_2) false))))

(fn `RemoveAllCards`
  (for _array_element (`self.cards`)
    (`ActorComponent.K2_DestroyComponent` _array_element))
  (`KismetArrayLibrary.Array_Clear` (`self.cards`))
  (`KismetArrayLibrary.Array_Clear` (`self.cardActors`)))

(fn `UpdateCardsScale`
  (bind _value (`/jnc/Observables/AC/jnc_AC_ObservableInt.Get` (`self.downIndex`)))
  (for (_array_element _array_index) (`self.cards`)
    (`SceneComponent.SetRelativeScale3D` _array_element (`KismetMathLibrary.VLerp` (`SceneComponent.RelativeScale3D` _array_element) (`KismetMathLibrary.Conv_DoubleToVector` (`KismetMathLibrary.SelectFloat` 1.1 1.0 (and (== _array_index _value) (!= _value -1)))) 0.2))))

(fn `UpdateHoverIndex`
  (bind _hitcomponent (`/Game/Art/jnc/TD/Blueprints/jnc_BP_TDPlayerController.hitComponent` (`/Game/Art/jnc/TD/Blueprints/jnc_BP_TD_Utils.TD PlayerController`)))
  ; Update only if no current "down" card
  (if (== (`/jnc/Observables/AC/jnc_AC_ObservableInt.Get` (`self.downIndex`)) -1)
    (`/Engine/EditorBlueprintResources/StandardMacros.IsValid` _hitcomponent
      (:`Is Valid`
        (`/jnc/Observables/AC/jnc_AC_ObservableInt.Set` (`self.hoverIndex`) (`self.GetHitCardIndex` _hitcomponent))))))

(fn `UserConstructionScript`
  (`self.CreateCards`))