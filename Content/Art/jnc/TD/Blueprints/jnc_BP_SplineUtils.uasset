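; Spline utility Blueprint whose RoundedSpline function rebuilds a Derived spline as a rounded-corner version of a Master spline.
; It clears Derived, copies the first point, adds two points per Master segment inset by Radius from each end, then appends the final point position.
; Inset points use custom tangents along the segment, scaled to twice Radius, so interior corners become curves, with one spline update at the end.
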(fn `RoundedSpline`
  (params (radius :type "Float (double-precision)" :default 50.0) (master :type "SplineComponent Object Reference") (derived :type "SplineComponent Object Reference"))
  (locals (count :type Integer :default 0) (delta :type "Vector Structure") (deltaLength :type "Float (double-precision)" :default 0.0) (direction :type "Vector Structure") (p0 :type "Vector Structure"))
  (bind _returnvalue (* (`local.direction`) (* (`local.radius`) 2.0)))
  (`|ExecutionSequence`
    (:`then_0`
      (set `local.count` (`SplineComponent.GetNumberOfSplinePoints` (`local.master`)))
      (`SplineComponent.ClearSplinePoints` (`local.derived`) false)
      ;[0.000911 0.004218 0.007812 0.5] First point
      (`SplineComponent.AddPoint` (`local.derived`) (`SplineComponent.GetSplinePointAt` (`local.master`) 0 "Local") false))
    (:`then_1`
      (for _index (range 1 (`local.count`))
        (bind (_returnvalue_inputkey _returnvalue_position) (break `SplinePoint` (`SplineComponent.GetSplinePointAt` (`local.master`) (- _index 1) "Local")))
        (set `local.p0` _returnvalue_position)
        (bind (_returnvalue_inputkey_2 _returnvalue_position_2) (break `SplinePoint` (`SplineComponent.GetSplinePointAt` (`local.master`) _index "Local")))
        (bind _returnvalue_2 (- _returnvalue_position_2 _returnvalue_position))
        (set `local.delta` _returnvalue_2)
        (bind _returnvalue_3 (`KismetMathLibrary.VSize` _returnvalue_2))
        (set `local.deltaLength` _returnvalue_3)
        (set `local.direction` (/ _returnvalue_2 _returnvalue_3))
        (`|ExecutionSequence`
          (:`then_0`
            (bind _returnvalue_4 (+ (* _index 2) -1))
            (`SplineComponent.AddPoint` (`local.derived`) (make `SplinePoint` (`KismetMathLibrary.Conv_IntToDouble` _returnvalue_4) (+ (`local.p0`) (* (`local.direction`) (`local.radius`))) _returnvalue _returnvalue (struct) (1.0 1.0 1.0) "CurveCustomTangent") false))
          (:`then_1`
            (`SplineComponent.AddPoint` (`local.derived`) (make `SplinePoint` (`KismetMathLibrary.Conv_IntToDouble` (+ _returnvalue_4 1)) (+ (`local.p0`) (* (`local.direction`) (- (`local.deltaLength`) (`local.radius`)))) _returnvalue _returnvalue (struct) (1.0 1.0 1.0) "CurveCustomTangent") false)))))
    (:`then_2`
      ;[0.000911 0.004218 0.007812 0.5] Last point
      (`SplineComponent.AddPoint` (`local.derived`) (make `SplinePoint` (`KismetMathLibrary.Conv_IntToDouble` (* (`local.count`) 2)) (`.Position` (break `SplinePoint` (`SplineComponent.GetSplinePointAt` (`local.master`) (- (`local.count`) 1) "Local")))) false))
    (:`then_3`
      (`SplineComponent.UpdateSpline` (`local.derived`)))))