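; Player controller for the TD mode that tracks the mouse cursor over the world and its pressed state.
; BeginPlay shows the cursor and adds the TD Enhanced Input mapping context, whose press action drives CursorIsDown.
; Each tick, a cursor trace stores the hit component and, on ground-channel hits, a grid-snapped location at zero height.
; It also feeds the press state into an observable bool and prints the mouse position for debugging.
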(event `self.ReceiveBeginPlay`
  (set `self.bShowMouseCursor` true)
  (set `self.bEnableClickEvents` true)
  (set `self.bEnableMouseOverEvents` true)
  (`EnhancedInputSubsystemInterface.AddMappingContext` (pcsubsystem `EnhancedInputLocalPlayerSubsystem` self) "/Game/Art/jnc/TD/jnc_IMC_TD.jnc_IMC_TD" 0 (struct)))

(event `self.ReceiveTick`
  (params (DeltaSeconds :type "Float (single-precision)"))
  (`self.UpdateCursor`)
  (bind _returnvalue (`WidgetLayoutLibrary.GetMousePositionOnViewport`))
  (`KismetSystemLibrary.PrintString` (`KismetStringLibrary.Conv_Vector2dToString` _returnvalue) true true (struct :`G` 0.66 :`B` 1.0 :`A` 1.0) 2.0 "m"))

(event `EnhancedInput|/Game/Art/jnc/TD/jnc_IA_TDCursorPressed`
  (params (ActionValue :type Boolean) (ElapsedSeconds :type "Float (double-precision)") (TriggeredSeconds :type "Float (double-precision)") (InputAction :type "InputAction Object Reference" :default "/Game/Art/jnc/TD/jnc_IA_TDCursorPressed.jnc_IA_TDCursorPressed"))
  (:`Triggered`
    (set `self._cursorIsDown` true :!label _label))
  (:`Started`
    (goto _label))
  (:`Canceled`
    (set `self._cursorIsDown` false :!label _label_2))
  (:`Completed`
    (goto _label_2)))

(fn `UpdateCursor`
  (bind (_hitresult _returnvalue) (`self.GetHitResultUnderCursorForObjects` (`|MakeArray` "ObjectTypeQuery7" "ObjectTypeQuery8" :!type "EObjectTypeQuery Enum") false))
  (bind (_bblockinghit _binitialoverlap _time _distance _location _impactpoint _normal _impactnormal _physmat _hitactor _hitcomponent) (`GameplayStatics.BreakHitResult` _hitresult))
  (bind (_result_x _result_y) (`KismetMathLibrary.BreakVector` (`/jnc/Library/jnc_BP_BasicUtils.FloorBy` _location 100.0)))
  (if _returnvalue
    (set `self.hitComponent` _hitcomponent)
    (if (`|EnumEquality` (`PrimitiveComponent.GetCollisionObjectType` _hitcomponent) "ECC_GameTraceChannel1")
      (set `self.cursorGroundLocation` (`KismetMathLibrary.MakeVector` _result_x _result_y))
      (set `self.cursorIsGround` true)
      (else
        (set `self.cursorIsGround` false :!label _label)))
    (else
      (set `self.hitComponent` null)
      (goto _label)))
  (`/jnc/Observables/jnc_ObservableBool.Set` (`self.cursorIsDown`) (`self._cursorIsDown`) -1.0))

(fn `UserConstructionScript`
  (bind _returnvalue (`|GenericCreateObject` "/jnc/Observables/jnc_ObservableBool.jnc_ObservableBool_C"))
  (set `self.cursorIsDown` _returnvalue))