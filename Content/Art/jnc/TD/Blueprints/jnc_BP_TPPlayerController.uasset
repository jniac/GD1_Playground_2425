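; Player controller for a TD input setup that provides mouse-driven cursor picking.
; On BeginPlay it shows the cursor, enables click and mouse-over events, and adds the TD Enhanced Input mapping context.
; The cursor-pressed input action runs a complex Visibility trace under the cursor and prints the hit actor's name, with no further action on the result.
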(event `self.ReceiveBeginPlay`
  (set `self.bShowMouseCursor` true)
  (set `self.bEnableClickEvents` true)
  (set `self.bEnableMouseOverEvents` true)
  (`EnhancedInputSubsystemInterface.AddMappingContext` (pcsubsystem `EnhancedInputLocalPlayerSubsystem` self) "/Game/jnc_IMC_TD.jnc_IMC_TD" 0 (struct)))

(event `EnhancedInput|/Game/Art/jnc/TD/jnc_IA_TDCursorPressed`
  (params (ActionValue :type Boolean) (ElapsedSeconds :type "Float (double-precision)") (TriggeredSeconds :type "Float (double-precision)") (InputAction :type "InputAction Object Reference" :default "/Game/Art/jnc/TD/jnc_IA_TDCursorPressed.jnc_IA_TDCursorPressed"))
  (:`Triggered`
    (`KismetSystemLibrary.PrintString` (`KismetSystemLibrary.GetDisplayName` (`.HitActor` (`GameplayStatics.BreakHitResult` (`self.GetHitResultUnderCursorByChannel` "TraceTypeQuery1")))))))

(fn `UserConstructionScript`)