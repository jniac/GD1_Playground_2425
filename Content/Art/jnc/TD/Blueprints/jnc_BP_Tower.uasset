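; Tower actor Blueprint in a TD folder, currently an early stub with no working tower logic.
; BeginPlay, the click event and the construction script are empty, and the cursor-over handler only prints a debug string, with its binding left disconnected.
; An unconnected construction-script chain would snap the actor's location to a 50-unit grid by dividing, rounding and multiplying back.
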(event `self.ReceiveBeginPlay`)

(event `OnOver` :!signature `self.OnBeginCursorOver`
  (params (TouchedActor :type "Actor Object Reference"))
  (`KismetSystemLibrary.PrintString` "over"))

(event `self.ReceiveActorOnClicked`
  (params (ButtonPressed :type "Key Structure")))

(fn `UserConstructionScript`)